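; Player controller for DestructionCity that routes all input across the building, mid-story, destruction and result scenes.
; It spawns and destroys a controller actor per scene, setting cursor and click settings, and forwards validity-checked input to it.
; Pause state gates building input and diverts gamepad navigation to the pause widget, otherwise to result handlers during results.
; Debug keys shorten the building timer or change the mayor's HP.
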(event `InputAction|GameEnd`
  (params (Key :type "Key Structure"))
  ;[1 0 0] ゲーム終了処理
)

(event `InputAction|Pause` :paused true
  (params (Key :type "Key Structure"))
  ;[1 1 1] ポーズ画面展開処理
  (:`Pressed`
    (`self.fChangePause`) ; カーソル関連の処理
    (`/Game/Pause/WBP_Pause.fChangeDraw` (`/Game/Play/Common/GameMode/GM_DestructionCity.mWBP_Pause` (cast `/Game/Play/Common/GameMode/GM_DestructionCity` (`GameplayStatics.GetGameMode`) :!pure true))) ; 表示切替処理
    (`GameplayStatics.SetGamePaused` false)))

(event `InputAction|GameStartButton` :paused true
  (params (Key :type "Key Structure"))
  ;[1 1 1] ゲームパッドで何かしらの項目で決定ボタンを押した処理
  (:`Pressed`
    (if (not (`self.GetPauseInactiveFlag`))
      (`self.PauseGamePadDecision`) ; ポーズメニューの決定処理
      (elif (`self.IsResult`)
        (`self.EventResultDecision`) ; リザルトの決定処理
      ))))

(event `Key|AnyKey` :paused true
  (params (Key :type "Key Structure"))
  ;[1 1 1] ゲームパッドでいずれかのボタンを押されたとき
  (:`Pressed`
    (if (`KismetInputLibrary.Key_IsGamepadKey` Key)
      (if (not (`self.GetPauseInactiveFlag`))
        (`self.PushPauseGamePadAnyKey`) ; ポーズメニューで何かしらのキーを押したときの処理
        (else
          (`self.ResetPauseGamePadAnyKey`) ; ポーズメニューでキーを押した判定をリセット
          (if (`self.IsResult`)
            (`self.ResultGamePadAnyKey`)
            (else
              (`self.ResetResultGamePadAnyKey`))))))))

(event `InputAction|SelectUp` :paused true
  (params (Key :type "Key Structure"))
  ;[1 1 1] ゲームパッドのキー操作処理
  (:`Pressed`
    (if (not (`self.GetPauseInactiveFlag`))
      (`self.PauseGamePadSelectUp`)
      (elif (`self.IsResult`)
        (`self.ResultSelectUp`)))))

(event `Key|Five`
  (params (Key :type "Key Structure"))
  (bind (_asgm_destruction_city _bsuccess) (cast `/Game/Play/Common/GameMode/GM_DestructionCity` (`GameplayStatics.GetGameMode`) :!pure true))
  (bind _mbp_buildingmanager (`/Game/Play/Common/GameMode/GM_DestructionCity.mBP_BuildingManager` _asgm_destruction_city))
  ;[0.9108 1 0] 建物建築シーン時間短縮デバッグ処理
  (:`Pressed`
    (if (and (`/Game/Play/Common/GameInstance/GMI_DestructionCIty.IsDEBUG` (cast `/Game/Play/Common/GameInstance/GMI_DestructionCIty` (`GameplayStatics.GetGameInstance`) :!pure true)) _bsuccess)
      (`/Engine/EditorBlueprintResources/StandardMacros.IsValid` _mbp_buildingmanager
        (:`Is Valid`
          (set `/Game/Play/Building/BP_BuildingManager.mTimeLimit` 4 _mbp_buildingmanager))))))

(event `InputAction|SelectDown` :paused true
  (params (Key :type "Key Structure"))
  ;[1 1 1] ゲームパッドのキー操作処理
  (:`Pressed`
    (if (not (`self.GetPauseInactiveFlag`))
      (`self.PauseGamePadSelectDown`)
      (elif (`self.IsResult`)
        (`self.ResultSelectDown`)))))

(event `InputAction|SelectLeft`
  (params (Key :type "Key Structure"))
  ;[1 1 1] ゲームパッドのキー操作処理
  (:`Pressed`
    (if (`self.IsResult`)
      (`self.ResultSelectLeft`))))

(event `InputAction|SelectRight`
  (params (Key :type "Key Structure"))
  ;[1 1 1] ゲームパッドのキー操作処理
  (:`Pressed`
    (if (`self.IsResult`)
      (`self.ResultSelectRight`))))

(event `InputAction|UpSoundGauge` :paused true
  (params (Key :type "Key Structure"))
  ;[1 1 1] ゲームパッド操作時の音量調整
  (:`Pressed`
    (if (not (`self.GetPauseInactiveFlag`))
      (switch `/Game/Pause/EN_Pause` (`self.IsInstructionActive`) ; 説明書が開いた状態かどうか
        (:`NewEnumerator1`
          (`/Game/Pause/WBP_Pause.GamePadChangeSoundVolume` (`self.GetWBP_Pause`) 0.1))))))

(event `InputAction|DownSoundGauge` :paused true
  (params (Key :type "Key Structure"))
  ;[1 1 1] ゲームパッド操作時の音量調整
  (:`Pressed`
    (if (not (`self.GetPauseInactiveFlag`))
      (switch `/Game/Pause/EN_Pause` (`self.IsInstructionActive`) ; 説明書が開いた状態かどうか
        (:`NewEnumerator1`
          (`/Game/Pause/WBP_Pause.GamePadChangeSoundVolume` (`self.GetWBP_Pause`) -0.1))))))

(event `InputAction|ShiftSelectBuildingRight`
  (params (Key :type "Key Structure"))
  (bind _mbp_buildingcontroller (`self.mBP_BuildingController`))
  ;[1 1 1] 横軸建物選択変更処理
  (:`Pressed`
    (if (`self.GetPauseInactiveFlag`)
      (if (`KismetSystemLibrary.IsValid` _mbp_buildingcontroller)
        (if (`/Game/Play/Building/BP_BuildingManager.mCasual` (`/Game/Play/Common/GameMode/GM_DestructionCity.mBP_BuildingManager` (cast `/Game/Play/Common/GameMode/GM_DestructionCity` (`GameplayStatics.GetGameMode`) :!pure true)))
          (`/Game/Play/Building/Controller/BP_BuildingController.F Casual Side Building Attributes` _mbp_buildingcontroller true)
          (else
            (`/Game/Play/Building/Controller/BP_BuildingController.F Side Building Attributes` _mbp_buildingcontroller true)))))))

(event `InputAction|ShiftSelectBuildingLeft`
  (params (Key :type "Key Structure"))
  (bind _mbp_buildingcontroller (`self.mBP_BuildingController`))
  ;[1 1 1] 横軸建物選択変更処理
  (:`Pressed`
    (if (`self.GetPauseInactiveFlag`)
      (if (`KismetSystemLibrary.IsValid` _mbp_buildingcontroller)
        (if (`/Game/Play/Building/BP_BuildingManager.mCasual` (`/Game/Play/Common/GameMode/GM_DestructionCity.mBP_BuildingManager` (cast `/Game/Play/Common/GameMode/GM_DestructionCity` (`GameplayStatics.GetGameMode`) :!pure true)))
          (`/Game/Play/Building/Controller/BP_BuildingController.F Casual Side Building Attributes` _mbp_buildingcontroller false)
          (else
            (`/Game/Play/Building/Controller/BP_BuildingController.F Side Building Attributes` _mbp_buildingcontroller false)))))))

(event `InputAction|Building`
  (params (Key :type "Key Structure"))
  (bind _mbp_buildingcontroller (`self.mBP_BuildingController`))
  ;[1 1 1] 建物建設処理
  (:`Pressed`
    (if (`self.GetPauseInactiveFlag`)
      (if (`KismetSystemLibrary.IsValid` _mbp_buildingcontroller)
        (`/Game/Play/Building/Controller/BP_BuildingController.fBuilding` _mbp_buildingcontroller)))))

(event `InputAxis|CameraMoveForward`
  (params (AxisValue :type "Float (single-precision)"))
  (bind _mbp_buildingcontroller (`self.mBP_BuildingController`))
  ;[1 1 1] カメラ移動処理
  (if (`self.GetPauseInactiveFlag`)
    (if (`KismetSystemLibrary.IsValid` _mbp_buildingcontroller)
      (`/Game/Play/Building/Controller/BP_BuildingController.fCameraMoveForward` _mbp_buildingcontroller AxisValue))))

(event `InputAxis|CameraMoveRight`
  (params (AxisValue :type "Float (single-precision)"))
  (bind _mbp_buildingcontroller (`self.mBP_BuildingController`))
  ;[1 1 1] カメラ移動処理
  (if (`self.GetPauseInactiveFlag`)
    (if (`KismetSystemLibrary.IsValid` _mbp_buildingcontroller)
      (`/Game/Play/Building/Controller/BP_BuildingController.fCameraMoveRight` _mbp_buildingcontroller AxisValue))))

(event `InputAction|SwitchLeftBuildingAttributes`
  (params (Key :type "Key Structure"))
  (bind _mbp_buildingcontroller (`self.mBP_BuildingController`))
  ;[1 1 1] 縦軸建物選択変更処理
  (:`Pressed`
    (if (`self.GetPauseInactiveFlag`)
      (if (`KismetSystemLibrary.IsValid` _mbp_buildingcontroller)
        (`/Game/Play/Building/Controller/BP_BuildingController.F Change Building Attributes Up` _mbp_buildingcontroller)))))

(event `InputAction|SwitchRightBuildingAttributes`
  (params (Key :type "Key Structure"))
  (bind _mbp_buildingcontroller (`self.mBP_BuildingController`))
  ;[1 1 1] 縦軸建物選択変更処理
  (:`Pressed`
    (if (`self.GetPauseInactiveFlag`)
      (if (`KismetSystemLibrary.IsValid` _mbp_buildingcontroller)
        (`/Game/Play/Building/Controller/BP_BuildingController.F Change Building Attributes Down` _mbp_buildingcontroller)))))

(event `InputAxis|PadMoveCursorForward`
  (params (AxisValue :type "Float (single-precision)"))
  (bind _mbp_buildingcontroller (`self.mBP_BuildingController`))
  ;[1 1 1] パッドのカーソル移動処理
  (if (`self.GetPauseInactiveFlag`)
    (if (`KismetSystemLibrary.IsValid` _mbp_buildingcontroller)
      (`/Game/Play/Building/Controller/BP_BuildingController.fMovePadCursorForward` _mbp_buildingcontroller AxisValue))))

(event `InputAxis|PadMoveCursorRight`
  (params (AxisValue :type "Float (single-precision)"))
  (bind _mbp_buildingcontroller (`self.mBP_BuildingController`))
  ;[1 1 1] パッドのカーソル移動処理
  (if (`self.GetPauseInactiveFlag`)
    (if (`KismetSystemLibrary.IsValid` _mbp_buildingcontroller)
      (`/Game/Play/Building/Controller/BP_BuildingController.fMovePadCursorRight` _mbp_buildingcontroller AxisValue))))

(event `InputAction|ChangeCamera`
  (params (Key :type "Key Structure"))
  (bind _returnvalue (`self.GetPauseInactiveFlag`))
  (bind _mbp_buildingcontroller (`self.mBP_BuildingController`))
  (bind _returnvalue_2 (`KismetSystemLibrary.IsValid` _mbp_buildingcontroller))
  (bind _returnvalue_3 (`|EnumEquality` (`/Game/Play/Common/GameMode/GM_DestructionCity.mGameState` (cast `/Game/Play/Common/GameMode/GM_DestructionCity` (`GameplayStatics.GetGameMode`) :!pure true)) "NewEnumerator0"))
  ;[1 1 1] カメラ視点切り替え処理
  (:`Pressed`
    (if _returnvalue
      (if _returnvalue_3
        (if _returnvalue_2
          (`/Game/Play/Building/Controller/BP_BuildingController.fChangeCamera` _mbp_buildingcontroller true)))))
  (:`Released`
    (if _returnvalue
      (if _returnvalue_3
        (if _returnvalue_2
          (`/Game/Play/Building/Controller/BP_BuildingController.fChangeCamera` _mbp_buildingcontroller false))))))

(event `Key|Six`
  (params (Key :type "Key Structure"))
  ;[1 0.7411 0] 市長のHPを少なくするデバッグ処理
  (:`Pressed`
    (if (`/Game/Play/Common/GameInstance/GMI_DestructionCIty.IsDEBUG` (cast `/Game/Play/Common/GameInstance/GMI_DestructionCIty` (`GameplayStatics.GetGameInstance`) :!pure true))
      (bind _asbp_mayor (cast `/Game/Play/Destruction/Mayor/BP_Mayor` (`GameplayStatics.GetPlayerCharacter` 0)))
      (set `/Game/Play/Destruction/Mayor/BP_Mayor.mHP` 3.0 _asbp_mayor))))

(event `InputAction|MayorForwardAttack`
  (params (Key :type "Key Structure"))
  (bind _mbp_destructioncontroller (`self.mBP_DestructionController`))
  ;[1 1 1] 市長の前方攻撃処理
  (:`Pressed`
    (`/Engine/EditorBlueprintResources/StandardMacros.IsValid` _mbp_destructioncontroller
      (:`Is Valid`
        (if (`/Game/Play/Destruction/BP_DestructionController.mIsOperable` _mbp_destructioncontroller)
          (set `self.mIsPressAttack` true) ; 攻撃ボタンを押しているフラグをtrueに
          (`/Game/Play/Destruction/BP_DestructionController.fMayorForwardAttack` _mbp_destructioncontroller) ; 前方攻撃処理
        ))))
  (:`Released`
    (`/Engine/EditorBlueprintResources/StandardMacros.IsValid` _mbp_destructioncontroller
      (:`Is Valid`
        (if (`/Game/Play/Destruction/BP_DestructionController.mIsOperable` _mbp_destructioncontroller)
          (`/Game/Play/Destruction/BP_DestructionController.F Mayor Attack` _mbp_destructioncontroller) ; 市長の攻撃処理
          (set `self.mIsPressAttack` false) ; 攻撃ボタンを押しているフラグをfalseに
        )))))

(event `InputAxis|MayorMoveForward`
  (params (AxisValue :type "Float (single-precision)"))
  (bind _mbp_destructioncontroller (`self.mBP_DestructionController`))
  ;[1 1 1] 市長の前進処理
  (`/Engine/EditorBlueprintResources/StandardMacros.IsValid` _mbp_destructioncontroller
    (:`Is Valid`
      (if (`/Game/Play/Destruction/BP_DestructionController.mIsOperable` _mbp_destructioncontroller)
        (if (not (`/Game/Play/Destruction/BP_DestructionController.mIsCharge` (`self.mBP_DestructionController`)))
          (`/Game/Play/Destruction/BP_DestructionController.fMayorMoveForward` _mbp_destructioncontroller AxisValue))))))

(event `InputAxis|MayorTurn`
  (params (AxisValue :type "Float (single-precision)"))
  (bind _mbp_destructioncontroller (`self.mBP_DestructionController`))
  ;[1 1 1] 市長の縦方向の視点処理
  (`/Engine/EditorBlueprintResources/StandardMacros.IsValid` _mbp_destructioncontroller
    (:`Is Valid`
      (if (`/Game/Play/Destruction/BP_DestructionController.mIsOperable` _mbp_destructioncontroller)
        (`/Game/Play/Destruction/BP_DestructionController.fMayorTurn` _mbp_destructioncontroller AxisValue)))))

(event `InputAxis|MayorLookUp`
  (params (AxisValue :type "Float (single-precision)"))
  (bind _mbp_destructioncontroller (`self.mBP_DestructionController`))
  ;[1 1 1] 市長の横方向の視点処理
  (`/Engine/EditorBlueprintResources/StandardMacros.IsValid` _mbp_destructioncontroller
    (:`Is Valid`
      (if (`/Game/Play/Destruction/BP_DestructionController.mIsOperable` _mbp_destructioncontroller)
        (`/Game/Play/Destruction/BP_DestructionController.fMayorLookUp` _mbp_destructioncontroller AxisValue)))))

(event `InputAxis|MayorMoveRight`
  (params (AxisValue :type "Float (single-precision)"))
  (bind _mbp_destructioncontroller (`self.mBP_DestructionController`))
  ;[1 1 1] 市長の左右の移動処理
  (`/Engine/EditorBlueprintResources/StandardMacros.IsValid` _mbp_destructioncontroller
    (:`Is Valid`
      (if (`/Game/Play/Destruction/BP_DestructionController.mIsOperable` _mbp_destructioncontroller)
        (if (not (`/Game/Play/Destruction/BP_DestructionController.mIsCharge` (`self.mBP_DestructionController`)))
          (`/Game/Play/Destruction/BP_DestructionController.fMayorMoveRight` _mbp_destructioncontroller AxisValue)
          (else
            (`self.MayorChargeTurn` AxisValue) ; 市長の溜め状態時の回転処理
          ))))))

(event `Key|Seven`
  (params (Key :type "Key Structure"))
  ;[1 0.7411 0] 市長のHPを多くするデバッグ処理
  (:`Pressed`
    (if (`/Game/Play/Common/GameInstance/GMI_DestructionCIty.IsDEBUG` (cast `/Game/Play/Common/GameInstance/GMI_DestructionCIty` (`GameplayStatics.GetGameInstance`) :!pure true))
      (bind _asbp_mayor (cast `/Game/Play/Destruction/Mayor/BP_Mayor` (`GameplayStatics.GetPlayerCharacter` 0)))
      (set `/Game/Play/Destruction/Mayor/BP_Mayor.mHP` 1000.0 _asbp_mayor))))

(event `InputAction|MayorLateralAttack`
  (params (Key :type "Key Structure"))
  (bind _mbp_destructioncontroller (`self.mBP_DestructionController`))
  ;[1 1 1] 市長の横方向攻撃処理
  (:`Pressed`
    (`/Engine/EditorBlueprintResources/StandardMacros.IsValid` _mbp_destructioncontroller
      (:`Is Valid`
        (if (`/Game/Play/Destruction/BP_DestructionController.mIsOperable` _mbp_destructioncontroller)
          (set `self.mIsPressAttack` true) ; 攻撃ボタンを押しているフラグをtrueに
          (`/Game/Play/Destruction/BP_DestructionController.fMayorLateralAttack` _mbp_destructioncontroller) ; 市長の横方向攻撃処理
        ))))
  (:`Released`
    (`/Engine/EditorBlueprintResources/StandardMacros.IsValid` _mbp_destructioncontroller
      (:`Is Valid`
        (if (`/Game/Play/Destruction/BP_DestructionController.mIsOperable` _mbp_destructioncontroller)
          (`/Game/Play/Destruction/BP_DestructionController.F Mayor Attack` _mbp_destructioncontroller) ; 市長の攻撃処理
          (set `self.mIsPressAttack` false) ; 攻撃ボタンを押しているフラグをfalseに
        )))))

(event `PlayFootSound`
  ;[1 1 1] 市長の足音を再生
  (`/Engine/EditorBlueprintResources/StandardMacros.DoOnce` false :!label _label
    (:`Completed`
      (`/Game/Play/Destruction/Sounds/BP_DestructionSoundManager.PlaySoundEffects` (`/Game/Play/Destruction/BP_DestructionManager.mBP_DestructionSoundManager` (`/Game/Play/Common/GameMode/GM_DestructionCity.mBP_DestructionManager` (`self.mGM_DestructionCity`))) null (0.0 0.0 0.0) 0.0)
      (`KismetSystemLibrary.Delay` 1.0)
      (goto _label :!via `Reset`))))

(event `MayorChargeTurn`
  (params (Value :type "Float (double-precision)"))
  ;[1 1 1] 市長の溜め状態時の回転処理
  (bind _asbp_mayor (cast `/Game/Play/Destruction/Mayor/BP_Mayor` (`GameplayStatics.GetPlayerCharacter` 0)))
  (bind (_returnvalue_roll _returnvalue_pitch _returnvalue_yaw) (`KismetMathLibrary.BreakRotator` (`self.K2_GetActorRotation` _asbp_mayor)))
  (`self.K2_SetActorRotation` _asbp_mayor (`KismetMathLibrary.MakeRotator` _returnvalue_roll _returnvalue_pitch (+ _returnvalue_yaw (* Value (`self.MAYOR_TURN_SPEED`)))) false))

(event `InputAction|Decision`
  (params (Key :type "Key Structure"))
  (bind _mbp_resultcontroller (`self.mBP_ResultController`))
  (bind _mbp_middlestorycontroller (`self.mBP_MiddleStoryController`))
  ;[1 1 1] ストーリーをスキップする
  (:`Pressed`
    (`/Engine/EditorBlueprintResources/StandardMacros.IsValid` _mbp_middlestorycontroller
      (:`Is Valid`
        (`/Game/Play/Story/BP_MiddleStoryController.SkipStory` _mbp_middlestorycontroller))
      (:`Is Not Valid`
        (`/Engine/EditorBlueprintResources/StandardMacros.IsValid` _mbp_resultcontroller
          (:`Is Valid`
            (`/Game/Result/BP_ResultController.SkipStory` _mbp_resultcontroller)))))))

(event `EventResultDecision`
  ;[1 1 1] リザルトでいずれかのモードを選択し押したときの処理
  (`/Game/Result/BP_ResultController.EndResultGamePad` (`self.mBP_ResultController`)))

(event `ResultGamePadAnyKey`
  ;[1 1 1] ゲームパッドでいずれかのボタンを押された際の処理
  (`/Engine/EditorBlueprintResources/StandardMacros.DoOnce` false :!label _label
    (:`Completed`
      (`/Game/Result/BP_ResultController.PushGamePadAnyKey` (`self.mBP_ResultController`)))))

(event `ResetResultGamePadAnyKey`
  ;[1 1 1] ゲームパッドでいずれかのボタンを押された際の処理
  (goto _label :!via `Reset`))

(event `ResultSelectUp`
  ;[1 1 1] リザルトシーンのキー操作処理
  (`/Game/Result/BP_ResultController.ResultSelectUp` (`self.mBP_ResultController`)))

(event `ResultSelectDown`
  ;[1 1 1] リザルトシーンのキー操作処理
  (`/Game/Result/BP_ResultController.ResultSelectDown` (`self.mBP_ResultController`)))

(event `ResultSelectRight`
  ;[1 1 1] リザルトシーンのキー操作処理
  (`/Game/Result/BP_ResultController.ResultSelectRight` (`self.mBP_ResultController`)))

(event `ResultSelectLeft`
  ;[1 1 1] リザルトシーンのキー操作処理
  (`/Game/Result/BP_ResultController.ResultSelectLeft` (`self.mBP_ResultController`)))

(event `PushPauseGamePadAnyKey`
  ;[1 1 1] ゲームパッドで何かしらのキーを押したとき
  (if (not (`self.GetPauseInactiveFlag`))
    (`/Game/Pause/WBP_Pause.PushGamePadAnyKey` (`self.GetWBP_Pause`))))

(event `PauseGamePadDecision`
  ;[1 1 1] ポーズメニューの決定処理
  (if (not (`self.GetPauseInactiveFlag`))
    (switch `/Game/Pause/EN_Pause` (`/Game/Pause/WBP_Pause.mInstructionsState` (`self.GetWBP_Pause`)) ; 説明書を開いた状態かどうか
      (:`NewEnumerator0`
        (`/Game/Pause/WBP_Pause.InstructionsReturn` (`self.GetWBP_Pause`)) ; 開いていたら説明書から戻る処理
      )
      (:`NewEnumerator1`
        (`/Game/Pause/WBP_Pause.fPauseDecision` (`self.GetWBP_Pause`)) ; 開いていないならポーズメニューの決定処理
      ))))

(event `PauseGamePadSelectUp`
  ;[1 1 1] ポーズメニューのキー操作処理
  (if (not (`self.GetPauseInactiveFlag`))
    (switch `/Game/Pause/EN_Pause` (`/Game/Pause/WBP_Pause.mInstructionsState` (`self.GetWBP_Pause`)) ; 説明書を開いた状態かどうか
      (:`NewEnumerator0`
        (`/Game/Pause/WBP_Pause.ShowInstructionsIconEmphasis` (`self.GetWBP_Pause`) "Visible"))
      (:`NewEnumerator1`
        (`/Game/Pause/WBP_Pause.fGamePadSelect` (`self.GetWBP_Pause`) -1)))))

(event `ResetPauseGamePadAnyKey`
  ;[1 1 1] ゲームパッドで何かしらのキーを押したとき
  (if (not (`self.GetPauseInactiveFlag`))
    (`/Game/Pause/WBP_Pause.ResetGamePadAnyKey` (`self.GetWBP_Pause`))))

(event `PauseGamePadSelectDown`
  ;[1 1 1] ポーズメニューのキー操作処理
  (if (not (`self.GetPauseInactiveFlag`))
    (switch `/Game/Pause/EN_Pause` (`/Game/Pause/WBP_Pause.mInstructionsState` (`self.GetWBP_Pause`)) ; 説明書を開いた状態かどうか
      (:`NewEnumerator0`
        (`/Game/Pause/WBP_Pause.ShowInstructionsIconEmphasis` (`self.GetWBP_Pause`) "Visible"))
      (:`NewEnumerator1`
        (`/Game/Pause/WBP_Pause.fGamePadSelect` (`self.GetWBP_Pause`) 1)))))

(fn `fChangePause`
  (if (`|EnumEquality` (`/Game/Play/Common/GameInstance/GMI_DestructionCIty.mPause` (cast `/Game/Play/Common/GameInstance/GMI_DestructionCIty` (`GameplayStatics.GetGameInstance`) :!pure true)) "NewEnumerator0")
    (switch `/Game/Play/Common/GameMode/EN_GameSate` (`/Game/Play/Common/GameMode/GM_DestructionCity.mGameState` (cast `/Game/Play/Common/GameMode/GM_DestructionCity` (`GameplayStatics.GetGameMode`) :!pure true))
      (:`NewEnumerator1`
        (set `self.bShowMouseCursor` false) ; マウスカーソルを消す
        (set `self.bEnableClickEvents` false) ; クリックイベントを無効に
        (set `self.ClickEventKeys` (`self.mDestructionClickKeys`)) ; 使用するキーを設定
      ))
    (else
      (set `self.bShowMouseCursor` true) ; マウスカーソルを表示する
      (set `self.bEnableClickEvents` true) ; クリックイベントを有効にする
      (set `self.ClickEventKeys` (`self.mBuildingClickKeys`)) ; 使用するキーを設定
    )))

(fn `fCreateBuildingController`
  ;[1 1 1] 各シーンのコントローラの作成
  (bind _returnvalue (`|SpawnActorFromClass` "/Game/Play/Building/Controller/BP_BuildingController.BP_BuildingController_C" (`KismetMathLibrary.MakeTransform` (0.0 0.0 0.0)) "Undefined" "OverrideRootScale" null null))
  (set `self.mBP_BuildingController` _returnvalue)
  (set `self.bShowMouseCursor` true) ; マウスカーソルを表示する
  (set `self.bEnableClickEvents` true) ; クリックイベントを有効にする
  (set `self.ClickEventKeys` (`self.mBuildingClickKeys`)) ; 使用するキーを設定
)

(fn `fCreateDestructionController`
  ;[1 1 1] 各シーンのコントローラの作成
  (bind _returnvalue (`|SpawnActorFromClass` "/Game/Play/Destruction/BP_DestructionController.BP_DestructionController_C" (`KismetMathLibrary.MakeTransform` (0.0 0.0 0.0)) "Undefined" "OverrideRootScale" null null))
  (set `self.mBP_DestructionController` _returnvalue)
  (set `self.bShowMouseCursor` false) ; マウスカーソルを表示する
  (set `self.bEnableClickEvents` false) ; クリックイベントを有効にする
  (set `self.ClickEventKeys` (`self.mDestructionClickKeys`)) ; 使用するキーを設定
)

(fn `fCreateMiddleStoryController`
  ;[1 1 1] 各シーンのコントローラの作成
  (bind _returnvalue (`|SpawnActorFromClass` "/Game/Play/Story/BP_MiddleStoryController.BP_MiddleStoryController_C" (`KismetMathLibrary.MakeTransform` (0.0 0.0 0.0)) "Undefined" "OverrideRootScale" null null))
  (set `self.mBP_MiddleStoryController` _returnvalue)
  (set `self.bShowMouseCursor` true) ; マウスカーソルを表示する
  (set `self.bEnableClickEvents` false) ; クリックイベントを有効にする
)

(fn `fCreateResultController`
  ;[1 1 1] 各シーンのコントローラの作成
  (bind _returnvalue (`|SpawnActorFromClass` "/Game/Result/BP_ResultController.BP_ResultController_C" (`KismetMathLibrary.MakeTransform` (0.0 0.0 0.0)) "Undefined" "OverrideRootScale" null null))
  (set `self.mBP_ResultController` _returnvalue)
  (set `self.bShowMouseCursor` false) ; マウスカーソルを表示する
  (set `self.bEnableClickEvents` false) ; クリックイベントを有効にする
)

(fn `fDeleteBuildingController`
  (bind _mbp_buildingcontroller (`self.mBP_BuildingController`))
  ;[1 1 1] 建物建築シーンのコントローラを削除
  (`/Engine/EditorBlueprintResources/StandardMacros.IsValid` _mbp_buildingcontroller
    (:`Is Valid`
      (`self.K2_DestroyActor` _mbp_buildingcontroller))))

(fn `fDeleteDestructionController`
  (bind _mbp_destructioncontroller (`self.mBP_DestructionController`))
  ;[1 1 1] 建物破壊シーンのコントローラを削除
  (`/Engine/EditorBlueprintResources/StandardMacros.IsValid` _mbp_destructioncontroller
    (:`Is Valid`
      (`self.K2_DestroyActor` _mbp_destructioncontroller))))

(fn `fDeleteMiddleStoryController`
  (bind _mbp_middlestorycontroller (`self.mBP_MiddleStoryController`))
  ;[1 1 1] 中盤ストーリーシーンのコントローラを削除
  (`/Engine/EditorBlueprintResources/StandardMacros.IsValid` _mbp_middlestorycontroller
    (:`Is Valid`
      (`self.K2_DestroyActor` _mbp_middlestorycontroller))))

(fn `fDeleteResultController`
  (bind _mbp_resultcontroller (`self.mBP_ResultController`))
  ;[1 1 1] 中盤ストーリーシーンのコントローラを削除
  (`/Engine/EditorBlueprintResources/StandardMacros.IsValid` _mbp_resultcontroller
    (:`Is Valid`
      (`self.K2_DestroyActor` _mbp_resultcontroller))))

(fn `UserConstructionScript`)