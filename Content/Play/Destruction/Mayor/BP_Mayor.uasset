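; Giant mayor character for the destruction scene, whose HP doubles as transformation time, draining outside bonus stages and on damage.
; A looping timer replaces Tick, handling the intro montage, one-time status-up multipliers and attack damage refresh.
; Attack state selects data-table damage and range plus montage, effect and sound for four attacks, with charging able to upgrade the state.
; Collision overlaps damage buildings and enemies, using global time dilation for hit stop on non-normal attacks.
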(event `self.ReceiveBeginPlay`
  ;[1 1 1] 初期化処理
  (`PrimitiveComponent.SetCollisionEnabled` (`self.AttackCollision`) "NoCollision")
  (set `self.mHP` (`self.INIT_HP`)) ; 市長の初期HPをセット
  (`self.fSet Mayor Attack Status`) ; 攻撃範囲を変更
  (`self.SetMayorSound`) ; 市長の必要な音をセット
  (`KismetSystemLibrary.K2_SetTimerDelegate` (delegate `Tick`) (`/Game/Play/Common/GameMode/GM_DestructionCity.DELTA_TIME` (cast `/Game/Play/Common/GameMode/GM_DestructionCity` (`GameplayStatics.GetGameMode`) :!pure true)) true))

(event `SetMayorSound`
  ;[1 1 1] 市長の必要な音をセット
  (`AudioComponent.SetSound` (`self.SoundMayorCharge`) "/Game/Play/Destruction/Sounds/SoundWave/Mayor/SoundEffect_MayorCharge.SoundEffect_MayorCharge")
  (`AudioComponent.SetSound` (`self.SoundHitMayorAttack`) "/Game/Play/Destruction/Sounds/SoundWave/Mayor/SoundEffect_HitMayorAttack.SoundEffect_HitMayorAttack"))

(event `Tick`
  ;[1 1 1] 更新処理
  (if (`|EnumEquality` (`/Game/Play/Common/GameMode/GM_DestructionCity.mGameState` (cast `/Game/Play/Common/GameMode/GM_DestructionCity` (`GameplayStatics.GetGameMode`) :!pure true)) "NewEnumerator1")
    (`self.BeginMayorAnimation`)
    (`self.SetMayorAttackStatus`) ; 市長の攻撃状態に応じた攻撃力をセット
    (`self.SpawnMayorStatusUpRatio`) ; 市長のステータスアップBPを生成
    (`self.DecreaseHP`) ; 市長のHPを徐々に減らす
    (`self.DestructionShowMayor`) ; 市長を破壊シーンならば表示する処理
  ))

(event `DecreaseHP`
  (bind _asgm_destruction_city (cast `/Game/Play/Common/GameMode/GM_DestructionCity` (`GameplayStatics.GetGameMode`) :!pure true))
  (bind _mbp_destructionmanager (`/Game/Play/Common/GameMode/GM_DestructionCity.mBP_DestructionManager` _asgm_destruction_city))
  (bind _mbp_bonusstagemanager (`/Game/Play/Destruction/BP_DestructionManager.mBP_BonusStageManager` _mbp_destructionmanager))
  ;[1 1 1] 市長のHPを徐々に減らす
  (`/Engine/EditorBlueprintResources/StandardMacros.IsValid` _mbp_destructionmanager
    (:`Is Valid`
      (`/Engine/EditorBlueprintResources/StandardMacros.IsValid` _mbp_bonusstagemanager
        (:`Is Valid`
          (if (not (`/Game/Play/Destruction/BonusStage/BP_BonusStageManager.mIsBonusStage` _mbp_bonusstagemanager))
            (set `self.mHP` (- (`self.mHP`) (`/Game/Play/Common/GameMode/GM_DestructionCity.DELTA_TIME` _asgm_destruction_city))) ; 市長のHPを減らす
          ))))))

(event `DestructionShowMayor`
  ;[1 1 1] 市長を破壊シーンならば表示する処理
  (`SceneComponent.SetVisibility` (`self.Mesh`) true false))

(event `MayorDamageDirection`
  ;[1 1 1] 市長のダメージ演出
  (bind (_direction `_新規track_0`) (`Timeline|DamageDirectionValue` :!via `PlayFromStart`)
    (:`Update`
      (`MeshComponent.SetVectorParameterValueOnMaterials` (`self.Mesh`) "DamageParam" (`KismetMathLibrary.MakeVector` `_新規track_0`)))))

(event `SpawnMayorStatusUpRatio`
  ;[1 1 1] 市長のステータスアップBPを生成
  (`/Engine/EditorBlueprintResources/StandardMacros.DoOnce` false
    (:`Completed`
      (`self.fSpawnMayorStatusUpRatio`))))

(event `SetMayorAttackStatus`
  ;[1 1 1] 市長の攻撃状態に応じた攻撃力をセット
  (`self.fSetMayorAttackDamage`) ; 市長の攻撃状態に応じた攻撃力をセット
)

(event `BeginMayorAnimation`
  ;[1 1 1] 破壊シーン最初の市長のアニメーション
  (`/Engine/EditorBlueprintResources/StandardMacros.DoOnce` false
    (:`Completed`
      (`self.PlayAnimMontage` "/Game/Play/Destruction/TitanAnim/ANIMM_MayorTitan.ANIMM_MayorTitan")
      (`KismetSystemLibrary.K2_SetTimerDelegate` (delegate `ResetMayorAnim`) (`self.BEGIN_ANIM_TIME`)))))

(event `ResetMayorAnim`
  ;[1 1 1] 破壊シーン最初の市長のアニメーション
  (`self.StopAnimMontage` "/Game/Play/Destruction/TitanAnim/ANIMM_MayorTitan.ANIMM_MayorTitan"))

(event `MayorNormalAttack`
  ;[1 1 1] 通常攻撃処理
  (`/Engine/EditorBlueprintResources/StandardMacros.DoOnce` false :!label _label
    (:`Completed`
      (`self.fMayorMontagePlay` "/Game/Play/Destruction/Mayor/Resources/Animations/NormalAttack/ANIMM_NormalAttack.ANIMM_NormalAttack" 1.0 0.0 true) ; アニメーションを再生
      (`self.fSpawnMayorAttackEffect` "/Game/UseEffect/P_MayorNormalAttack.P_MayorNormalAttack") ; 市長の攻撃エフェクトのトランスフォームを返す
      (`self.fPlayMayorAttackSound` "/Game/Play/Destruction/Sounds/SoundWave/Mayor/SoundEffect_MayorNormalAttack.SoundEffect_MayorNormalAttack") ; 効果音を再生
      (bind _mayordatatable (`self.fGetMayorAttackData`)) ; 市長の攻撃データを取得
      (`KismetSystemLibrary.Delay` (`.AttackInterval_4_8FE35EC143501DC2E5D9FCACA524E3CA` (break `/Game/Play/Destruction/Mayor/Data/ST_MayorDataTable` _mayordatatable)))
      (goto _label :!via `Reset`))))

(event `MayorChage`
  (bind _soundmayorcharge (`self.SoundMayorCharge`))
  ;[1 1 1] 溜め処理
  (`PrimitiveComponent.SetCollisionEnabled` (`self.AttackCollision`) "NoCollision") ; 攻撃の当たり判定を消す
  (`self.fMayorMontagePlay` "/Game/Play/Destruction/Mayor/Resources/Animations/Charge/ANIMM_MayorCharge.ANIMM_MayorCharge" 1.0 0.0 true) ; アニメーションを再生
  (`KismetSystemLibrary.Delay` (`self.CHARGE_SLOW_START_TIME`)) ; スローにするタイミングを遅らせる
  (`AnimInstance.Montage_SetPlayRate` (`SkeletalMeshComponent.GetAnimInstance` (`self.Mesh`)) "/Game/Play/Destruction/Mayor/Resources/Animations/Charge/ANIMM_MayorCharge.ANIMM_MayorCharge" (`self.CHARGE_SLOW_PLAY_RATE`)) ; スロー再生
  (`self.SpawnMayorChargeEffect`) ; 溜め状態エフェクトを生成
  (set `AudioComponent.VolumeMultiplier` (`/Game/Play/Destruction/Sounds/BP_DestructionSoundManager.mSoundEffectVolume` (`/Game/Play/Destruction/BP_DestructionManager.mBP_DestructionSoundManager` (`/Game/Play/Common/GameMode/GM_DestructionCity.mBP_DestructionManager` (cast `/Game/Play/Common/GameMode/GM_DestructionCity` (`GameplayStatics.GetGameMode`) :!pure true)))) _soundmayorcharge)
  (`AudioComponent.Play` _soundmayorcharge 0.0) ; 溜め状態の音を再生
)

(event `self.AttackCollision.OnComponentBeginOverlap`
  (params (OverlappedComponent :type "PrimitiveComponent Object Reference") (OtherActor :type "Actor Object Reference") (OtherComp :type "PrimitiveComponent Object Reference") (OtherBodyIndex :type Integer) (bFromSweep :type Boolean) (SweepResult :type "HitResult Structure (by ref)"))
  ;[1 1 1] 市長の攻撃当たり判定に触れた際の処理
  (`self.AttackCollisionHitBuilding` OtherActor) ; 攻撃コリジョンが建物にヒットした際の処理
  (`self.AttackCollisionHitEnemy` OtherActor) ; 攻撃コリジョンが敵にヒットした際の処理
)

(event `MayorAttack`
  ;[1 1 1] 市長の攻撃処理
  (`self.fSet Mayor Attack Status`) ; 攻撃範囲を変更
  (`self.fCalculateAttackDamage`) ; 攻撃倍率を加算した攻撃ダメージを計算
  (`self.fPlayAttackVoice`) ; 攻撃する際の市長の声を再生
  (switch `/Game/Play/Destruction/Mayor/Data/EN_MayorAttackState` (`self.mEN_MayorAttackState`) ; 市長の攻撃状態に応じて処理を変える
    (:`NewEnumerator0`
      (`self.MayorNormalAttack`) ; 通常攻撃処理
    )
    (:`NewEnumerator1`
      (`self.MayorFireKick`) ; 炎キック攻撃処理
    )
    (:`NewEnumerator2`
      (`self.MayorMowingAttack`) ; 薙ぎ払い攻撃処理
    )
    (:`NewEnumerator3`
      (`self.MayorChargeAttack`) ; 突進攻撃処理
    )))

(event `MayorFireKick`
  ;[1 1 1] 炎キック攻撃処理
  (`/Engine/EditorBlueprintResources/StandardMacros.DoOnce` false :!label _label_2
    (:`Completed`
      (`self.fMayorMontagePlay` "/Game/Play/Destruction/Mayor/Resources/Animations/FireKick/ANIMM_FireKick.ANIMM_FireKick" 1.0 0.0 true) ; アニメーションを再生
      (`self.fSpawnMayorAttackEffect` "/Game/UseEffect/P_MayorFireKick.P_MayorFireKick") ; 市長の攻撃エフェクトのトランスフォームを返す
      (`self.fPlayMayorAttackSound` "/Game/Play/Destruction/Sounds/SoundWave/Mayor/SoundEffect_FireKick.SoundEffect_FireKick") ; 効果音を再生
      (bind _mayordatatable (`self.fGetMayorAttackData`)) ; 市長の攻撃データを取得
      (`KismetSystemLibrary.Delay` (`.AttackInterval_4_8FE35EC143501DC2E5D9FCACA524E3CA` (break `/Game/Play/Destruction/Mayor/Data/ST_MayorDataTable` _mayordatatable)))
      (goto _label_2 :!via `Reset`))))

(event `AttackCollisionHitBuilding`
  (params (hitActor :type "Actor Object Reference"))
  ;[1 1 1] 攻撃コリジョンが建物にヒットした際の処理
  (bind _asbp_building_base (cast `/Game/Play/Building/BP_Building/BP_BuildingBase` hitActor))
  (if (`|EnumInequality` (`/Game/Play/Building/BP_Building/BP_BuildingBase.mBuilding` _asbp_building_base) "NewEnumerator13")
    (`self.fPlaySoundHitMayorAttack`) ; 市長の攻撃がヒットした時の音の再生処理
    (`/Game/Play/Building/BP_Building/BP_BuildingBase.BuildingApplyDamage` _asbp_building_base (`self.mMayorAttackDamage`) (`self.GetActorForwardVector`) 10000.0) ; 建物にダメージを当てる
    (`/Game/Play/Building/BP_Building/BP_BuildingBase.WoodenBuildingSpreadOfFire` _asbp_building_base (`self.mEN_MayorAttackState`)) ; 木材の建物の延焼処理
    (`self.HitStop` 0.2 0.05)
    (`self.SpawnObjectHitAttackEffect`) ; オブジェクトに当たった際の攻撃エフェクトを生成
  ))

(event `MayorForwardAttack`
  ;[1 1 1] 前方攻撃処理
  (set `self.mEN_MayorAttackState` "NewEnumerator0"))

(event `SpawnMayorChargeEffect`
  (bind (_returnvalue_location _returnvalue_rotation _returnvalue_scale) (`KismetMathLibrary.BreakTransform` (`self.GetTransform`)))
  (bind _mmayorchargeeffect (`self.mMayorChargeEffect`))
  ;[1 1 1] 溜め状態エフェクトを生成
  (bind _returnvalue (`GameplayStatics.SpawnEmitterAtLocation` "/Game/UseEffect/P_MayorCharge.P_MayorCharge" _returnvalue_location _returnvalue_rotation _returnvalue_scale)) ; 溜め状態エフェクトを生成
  (set `self.mMayorChargeEffect` _returnvalue)
  (bind (_direction `_新規track_0`) (`Timeline|タイムライン_0` :!via `PlayFromStart`)
    (:`Update`
      (`/Engine/EditorBlueprintResources/StandardMacros.IsValid` _mmayorchargeeffect
        (:`Is Valid`
          (`SceneComponent.SetWorldScale3D` _mmayorchargeeffect (* _returnvalue_scale `_新規track_0`)) ; スケールを加算
        )))))

(event `MayorLateralAttack`
  ;[1 1 1] 横方向攻撃処理
  (set `self.mEN_MayorAttackState` "NewEnumerator2"))

(event `MayorMowingAttack`
  ;[1 1 1] 薙ぎ払い攻撃処理
  (`/Engine/EditorBlueprintResources/StandardMacros.DoOnce` false :!label _label_3
    (:`Completed`
      (`self.fMayorMontagePlay` "/Game/Play/Destruction/Mayor/Resources/Animations/MowingAttack/ANIMM_MowingAttack.ANIMM_MowingAttack" 1.0 0.0 true) ; アニメーションを再生
      (`self.fSpawnMayorAttackEffect` "/Game/UseEffect/P_MayorMowingDownAttack.P_MayorMowingDownAttack") ; 市長の攻撃エフェクトのトランスフォームを返す
      (`self.fPlayMayorAttackSound` "/Game/Play/Destruction/Sounds/SoundWave/Mayor/SoundEffect_MayorMowingDownAttack.SoundEffect_MayorMowingDownAttack") ; 効果音を再生
      (bind _mayordatatable (`self.fGetMayorAttackData`)) ; 市長の攻撃データを取得
      (`KismetSystemLibrary.Delay` (`.AttackInterval_4_8FE35EC143501DC2E5D9FCACA524E3CA` (break `/Game/Play/Destruction/Mayor/Data/ST_MayorDataTable` _mayordatatable)))
      (goto _label_3 :!via `Reset`))))

(event `AttackCollisionHitEnemy`
  (params (HitActor :type "Actor Object Reference"))
  ;[1 1 1] 攻撃コリジョンが敵にヒットした際の処理
  (bind _asbp_enemy_base (cast `/Game/Play/Destruction/Enemy/BP_EnemyBase` HitActor))
  (`self.fPlaySoundHitMayorAttack`) ; 市長の攻撃がヒットした時の音の再生処理
  (`/Game/Play/Destruction/Enemy/BP_EnemyBase.EnemyApplyDamage` _asbp_enemy_base (`self.mMayorAttackDamage`) (`self.GetActorForwardVector`))
  (`self.HitStop` 0.2 0.05)
  (`self.SpawnObjectHitAttackEffect`) ; オブジェクトに当たった際の攻撃エフェクトを生成
)

(event `MayorChargeAttack`
  ;[1 1 1] 突進攻撃処理
  (`/Engine/EditorBlueprintResources/StandardMacros.DoOnce` false :!label _label_4
    (:`Completed`
      (`self.fMayorMontagePlay` "/Game/Play/Destruction/Mayor/Resources/Animations/ChargeAttack/ANIMM_ChargeAttack.ANIMM_ChargeAttack" 1.0 0.0 true) ; アニメーションを再生
      (`self.fSpawnMayorAttackEffect` "/Game/UseEffect/P_MayorChargeAttack.P_MayorChargeAttack") ; 市長の攻撃エフェクトのトランスフォームを返す
      (`self.fPlayMayorAttackSound` "/Game/Play/Destruction/Sounds/SoundWave/Mayor/SoundEffect_MayorChargeAttack.SoundEffect_MayorChargeAttack") ; 効果音を再生
      (bind _mayordatatable (`self.fGetMayorAttackData`)) ; 市長の攻撃データを取得
      (`KismetSystemLibrary.Delay` (`.AttackInterval_4_8FE35EC143501DC2E5D9FCACA524E3CA` (break `/Game/Play/Destruction/Mayor/Data/ST_MayorDataTable` _mayordatatable)))
      (goto _label_4 :!via `Reset`))))

(event `HitStop`
  (params (HitStopFrame :type "Float (double-precision)") (Delay :type "Float (double-precision)"))
  ;[1 1 1] ヒットストップ処理
  (if (and (not (`self.mHitStopFlag`)) (`|EnumInequality` (`self.mEN_MayorAttackState`) "NewEnumerator0"))
    (set `self.mHitStopFlag` true)
    (`GameplayStatics.SetGlobalTimeDilation` HitStopFrame)
    (`KismetSystemLibrary.K2_SetTimerDelegate` (delegate `ResetGlobalTime`) Delay)))

(event `ResetGlobalTime`
  ;[1 1 1] ヒットストップ処理
  (`GameplayStatics.SetGlobalTimeDilation` 1.0)
  (set `self.mHitStopFlag` false))

(event `SpawnObjectHitAttackEffect`
  (bind (_returnvalue_location _returnvalue_rotation) (`KismetMathLibrary.BreakTransform` (`SceneComponent.K2_GetComponentToWorld` (`self.AttackEffectPos`))))
  ;[1 1 1] オブジェクトに当たった際の攻撃エフェクトを生成
  (`GameplayStatics.SpawnEmitterAtLocation` "/Game/UseEffect/P_ObjectHit.P_ObjectHit" _returnvalue_location _returnvalue_rotation))

(fn `fAddAttackRate`
  (params (AddAttackRate :type "Float (double-precision)"))
  (locals (AddAttackRate_ :type "Float (double-precision)") (NowAttackRate :type "Float (double-precision)"))
  ;[1 1 1] 攻撃倍率を加算
  (set `self.mAttackRate` (+ AddAttackRate (`self.mDefaultAttackRate`))))

(fn `fCalculateAttackDamage`
  ;[1 1 1] 攻撃倍率を加算した攻撃ダメージを計算
  (set `self.mMayorAttackDamage` (`KismetMathLibrary.Conv_IntToDouble` (`KismetMathLibrary.Round` (* (`self.mMayorAttackDamage`) (`self.mAttackRate`))))) ; 攻撃ダメージをセット
)

(fn `fCheckHPWarning`
  (returns (IsWarning :type Boolean))
  ;[1 1 1] HPが警告が出るHP量以下か調べる
  (return (<= (`self.mHP`) (* (`self.INIT_HP`) (`self.WARNING_HP`)))))

(fn `fGetMayorAttackData`
  (returns (MayorDataTable :type "/Game/Play/Destruction/Mayor/Data/ST_MayorDataTable Structure"))
  ;[1 1 1] 市長の攻撃状態に対応するデータの取得
  (bind _asgm_destruction_city (cast `/Game/Play/Common/GameMode/GM_DestructionCity` (`GameplayStatics.GetGameMode`)))
  (bind _mbp_mayorattackdatatablemanager (`/Game/Play/Destruction/BP_DestructionManager.mBP_MayorAttackDataTableManager` (`/Game/Play/Common/GameMode/GM_DestructionCity.mBP_DestructionManager` _asgm_destruction_city)))
  (`/Engine/EditorBlueprintResources/StandardMacros.IsValid` _mbp_mayorattackdatatablemanager
    (:`Is Valid`
      (bind _mayordatatable (`/Game/Play/Destruction/Mayor/Data/BP_MayorAttackDataTableManager.fMap` _mbp_mayorattackdatatablemanager (`self.mEN_MayorAttackState`))) ; 攻撃状態に応じたデータテーブルを取得
      (return _mayordatatable))))

(fn `fIsDead`
  (returns (IsDead :type Boolean))
  ;[1 1 1] 市長の巨人化の時間が切れたか
  (return (<= (`self.mHP`) 0.0)))

(fn `fMaxChargeAttack`
  ;[1 1 1] 最大まで溜めた際攻撃の状態を変更する
  (if (`|EnumEquality` (`self.mEN_MayorAttackState`) "NewEnumerator0")
    (set `self.mEN_MayorAttackState` "NewEnumerator3")
    (elif (`|EnumEquality` (`self.mEN_MayorAttackState`) "NewEnumerator2")
      (set `self.mEN_MayorAttackState` "NewEnumerator1"))))

(fn `fMayorDamage`
  (params (Damage :type "Float (double-precision)"))
  ;[1 1 1] 市長にダメージを与える
  (set `self.mHP` (- (`self.mHP`) Damage))
  (`/Game/Play/Destruction/Sounds/BP_DestructionSoundManager.PlaySoundEffects` (`/Game/Play/Destruction/BP_DestructionManager.mBP_DestructionSoundManager` (`/Game/Play/Common/GameMode/GM_DestructionCity.mBP_DestructionManager` (cast `/Game/Play/Common/GameMode/GM_DestructionCity` (`GameplayStatics.GetGameMode`) :!pure true))) "/Game/Play/Destruction/Sounds/SoundWave/Mayor/SoundEffect_MayorDamage.SoundEffect_MayorDamage" (0.0 0.0 0.0) 0.0) ; 市長がダメージを受けた際の効果音を再生
  (`self.fPlayDamageVoice`) ; ダメージを受けた際の市長の声を再生
  (`self.MayorDamageDirection`) ; 市長のダメージ演出
)

(fn `fMayorMontagePlay`
  (params (AnimMontage :type "AnimMontage Object Reference") (InPlayRate :type "Float (double-precision)") (StartMontageTime :type "Float (double-precision)") (IsStopAllMontage :type Boolean))
  ;[1 1 1] 市長のアニメーションモンタージュを再生
  (`AnimInstance.Montage_Play` (`SkeletalMeshComponent.GetAnimInstance` (`self.Mesh`)) AnimMontage InPlayRate "MontageLength" StartMontageTime IsStopAllMontage) ; アニメーションを再生
)

(fn `fPlayAttackVoice`
  (locals (AttackVoice :type "SoundBase Object Reference"))
  ;[1 1 1] 攻撃する際の市長の声を再生
  (`/Engine/EditorBlueprintResources/StandardMacros.FlipFlop`
    (:`A`
      (set `local.AttackVoice` "/Game/Play/Destruction/Sounds/SoundWave/Mayor/SoundEffect_MayorAttackVoice1.SoundEffect_MayorAttackVoice1"))
    (:`B`
      (set `local.AttackVoice` "/Game/Play/Destruction/Sounds/SoundWave/Mayor/SoundEffect_MayorAttackVoice3.SoundEffect_MayorAttackVoice3")))
  (`/Game/Play/Destruction/Sounds/BP_DestructionSoundManager.PlaySoundEffects` (`self.GetSoundManager`) (`local.AttackVoice`) (0.0 0.0 0.0) 0.0))

(fn `fPlayDamageVoice`
  (locals (DamageVoice :type "SoundBase Object Reference"))
  ;[1 1 1] ダメージを受けた際の市長の声を再生
  (`/Engine/EditorBlueprintResources/StandardMacros.FlipFlop`
    (:`A`
      (set `local.DamageVoice` "/Game/Play/Destruction/Sounds/SoundWave/Mayor/SoundEffect_MayorDamageVoice1.SoundEffect_MayorDamageVoice1"))
    (:`B`
      (set `local.DamageVoice` "/Game/Play/Destruction/Sounds/SoundWave/Mayor/SoundEffect_MayorDamageVoice2.SoundEffect_MayorDamageVoice2")))
  (`/Game/Play/Destruction/Sounds/BP_DestructionSoundManager.PlaySoundEffects` (`self.GetSoundManager`) (`local.DamageVoice`) (0.0 0.0 0.0) 0.0))

(fn `fPlayMayorAttackSound`
  (params (SoundEffect :type "SoundBase Object Reference"))
  ;[1 1 1] 市長の攻撃効果音を再生
  (`/Game/Play/Destruction/Sounds/BP_DestructionSoundManager.PlaySoundEffects` (`/Game/Play/Destruction/BP_DestructionManager.mBP_DestructionSoundManager` (`/Game/Play/Common/GameMode/GM_DestructionCity.mBP_DestructionManager` (cast `/Game/Play/Common/GameMode/GM_DestructionCity` (`GameplayStatics.GetGameMode`) :!pure true))) SoundEffect (0.0 0.0 0.0) 0.0))

(fn `fPlaySoundHitMayorAttack`
  (bind _soundhitmayorattack (`self.SoundHitMayorAttack`))
  ;[1 1 1] 市長の攻撃がヒットした時の音の再生処理
  (if (not (`AudioComponent.IsPlaying` (`self.SoundHitMayorAttack`)))
    (set `AudioComponent.VolumeMultiplier` (`/Game/Play/Destruction/Sounds/BP_DestructionSoundManager.mSoundEffectVolume` (`/Game/Play/Destruction/BP_DestructionManager.mBP_DestructionSoundManager` (`/Game/Play/Common/GameMode/GM_DestructionCity.mBP_DestructionManager` (cast `/Game/Play/Common/GameMode/GM_DestructionCity` (`GameplayStatics.GetGameMode`) :!pure true)))) _soundhitmayorattack)
    (`AudioComponent.Play` _soundhitmayorattack 0.0) ; 攻撃がヒットした時の音を再生
  ))

(fn `fResetAttackRate`
  ;[1 1 1] 攻撃倍率をリセット
  (set `self.mMayorAttackDamage` (/ (`self.mMayorAttackDamage`) (`self.mAttackRate`))) ; 攻撃ダメージをリセット
  (set `self.mAttackRate` (`self.mDefaultAttackRate`)) ; 攻撃割合をリセット
)

(fn `fResetChargeEffect`
  (bind _mmayorchargeeffect (`self.mMayorChargeEffect`))
  ;[1 1 1] 溜め状態エフェクトを削除
  (`/Engine/EditorBlueprintResources/StandardMacros.IsValid` _mmayorchargeeffect
    (:`Is Valid`
      (`ActorComponent.K2_DestroyComponent` _mmayorchargeeffect))))

(fn `fSet Mayor Attack Status`
  ;[1 1 1] 市長の攻撃範囲を変更
  (bind _mayordatatable (`self.fGetMayorAttackData`)) ; 市長のデータを取得
  (set `self.mEN_MayorAttackState` (break `/Game/Play/Destruction/Mayor/Data/ST_MayorDataTable` _mayordatatable))
  (set `self.mMayorAttackDamage` (`.AttackDamage_2_E546B2E64A3C9C36C045FD9E33E85A4A` (break `/Game/Play/Destruction/Mayor/Data/ST_MayorDataTable` _mayordatatable)))
  (bind (_x _y) (`KismetMathLibrary.BreakVector2D` (`.AttackRange_11_7E7D60674AAA7896633DFDAFE4BEAFA0` (break `/Game/Play/Destruction/Mayor/Data/ST_MayorDataTable` _mayordatatable))))
  (`SceneComponent.SetWorldScale3D` (`self.AttackCollision`) (`KismetMathLibrary.MakeVector` (* _x (.x (`self.DEFAULT_ATTACK_RANGE`))) (* _y (.y (`self.DEFAULT_ATTACK_RANGE`))) (.z (`self.DEFAULT_ATTACK_RANGE`))))
  (`SceneComponent.SetWorldScale3D` (`self.AttackRangeCollision`) (`KismetMathLibrary.MakeVector` (* _x (.x (`self.DEFAULT_ATTACK_RANGE`))) (* _y (.y (`self.DEFAULT_ATTACK_RANGE`))) (.z (`self.DEFAULT_ATTACK_RANGE`)))) ; 攻撃範囲をセット
)

(fn `fSetMayorAttackDamage`
  ;[1 1 1] 市長の攻撃状態に応じた攻撃力をセット
  (bind _mayordatatable (`self.fGetMayorAttackData`))
  (set `self.mEN_MayorAttackState` (break `/Game/Play/Destruction/Mayor/Data/ST_MayorDataTable` _mayordatatable))
  (set `self.mMayorAttackDamage` (`.AttackDamage_2_E546B2E64A3C9C36C045FD9E33E85A4A` (break `/Game/Play/Destruction/Mayor/Data/ST_MayorDataTable` _mayordatatable))) ; 攻撃倍率を加算した状態の攻撃ダメージをセット
)

(fn `fSpawnMayorAttackEffect`
  (params (SpawnEffect :type "ParticleSystem Object Reference"))
  (locals (ST_MayorAttackEffectTransform :type "/Game/Play/Destruction/Mayor/Data/ST_MayorAttackEffectTransform Structure"))
  (bind _st_mayorattackeffecttransform_mayorattackeffecttransform (break `/Game/Play/Destruction/Mayor/Data/ST_MayorAttackEffectTransform` (`local.ST_MayorAttackEffectTransform`)))
  (bind (_value _returnvalue) (`BlueprintMapLibrary.Map_Find` _st_mayorattackeffecttransform_mayorattackeffecttransform (`self.mEN_MayorAttackState`)))
  (bind (_returnvalue_location _returnvalue_rotation _returnvalue_scale) (`KismetMathLibrary.BreakTransform` (`SceneComponent.K2_GetComponentToWorld` (`self.AttackEffectPos`))))
  (bind (_returnvalue_location_2 _returnvalue_rotation_2 _returnvalue_scale_2) (`KismetMathLibrary.BreakTransform` (`KismetMathLibrary.MakeTransform` (+ (.location _value) _returnvalue_location) (`KismetMathLibrary.MakeRotator` (+ (.roll (.rotation _value)) (.roll (`self.K2_GetActorRotation`))) (+ (.pitch (.rotation _value)) (.pitch (`self.K2_GetActorRotation`))) (+ (.yaw (.rotation _value)) (.yaw (`self.K2_GetActorRotation`)))) (* (+ (.scale _value) _returnvalue_scale) (`self.mAttackRate`)))))
  ;[1 1 1] 市長の攻撃エフェクトを生成
  (if _returnvalue
    (`GameplayStatics.SpawnEmitterAtLocation` SpawnEffect _returnvalue_location_2 _returnvalue_rotation_2 _returnvalue_scale_2)))

(fn `fSpawnMayorStatusUpRatio`
  ;[1 1 1] 市長のステータスアップBPを生成
  (bind _returnvalue (`|SpawnActorFromClass` "/Game/Play/Destruction/StatusUp/BP_MayorStatusUpRatio.BP_MayorStatusUpRatio_C" (`KismetMathLibrary.MakeTransform` (0.0 0.0 0.0)) "Undefined" "OverrideRootScale" null null)) ; 市長のステータスUPのBPを生成
  (bind _output_get (set `self.mBP_MayorStatusUpRatio` _returnvalue))
  (bind _hpupratio (`/Game/Play/Destruction/StatusUp/BP_MayorStatusUpRatio.fGetMayorHPUpRatio` _output_get))
  (set `self.mHP` (* (`self.mHP`) _hpupratio)) ; HPの倍率をセット
  (bind _attackdamageupratio (`/Game/Play/Destruction/StatusUp/BP_MayorStatusUpRatio.fGetMayorAttackDamageUpRatio` (`self.mBP_MayorStatusUpRatio`)))
  (set `self.mDefaultAttackRate` (* (`self.mDefaultAttackRate`) _attackdamageupratio)) ; デフォルト攻撃力の倍率をセット
)

(fn `UserConstructionScript`)